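; Gate Blueprint that players open and close by interacting, with a prompt widget shown while the player character overlaps its trigger box.
; The Interact3 function picks open or close from IsOpen and sets the timeline play rate from the matching duration.
; One timeline, played forward or reversed, lerps the gate's relative location between closed and open positions, toggling IsOpen only when it finishes.
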(event OnComponentBeginOverlap(box_0)
  (params (OverlappedComponent :type Primitive%20Component%20Object%20Reference) (OtherActor :type Actor%20Object%20Reference) (OtherComp :type Primitive%20Component%20Object%20Reference) (OtherBodyIndex :type Integer) (bFromSweep :type Boolean) (SweepResult :type Hit%20Result%20Structure%20%28by%20ref%29))
  ;[1 1 1] display text
  (if (== OtherActor (Game|GetPlayerCharacter 0))
    (UserInterface|Viewport|AddtoViewport (Variables|Default|GetInteract%20prompt) 0)))

(event OnComponentEndOverlap(box_0)
  (params (OverlappedComponent :type Primitive%20Component%20Object%20Reference) (OtherActor :type Actor%20Object%20Reference) (OtherComp :type Primitive%20Component%20Object%20Reference) (OtherBodyIndex :type Integer))
  ;[1 1 1] display text
  (if (== (Game|GetPlayerCharacter 0) OtherActor)
    (Widget|RemovefromParent (Variables|Default|GetInteract%20prompt))))

(event Custom|Open%20Door
  (bind _door (Timeline|open%20Door1 Play)
    (:Update
      (Transformation|SetRelativeLocation (Variables|Default|Getgate) (Math|Conversions|ToVector(Float) (Math|Float|Lerp (Variables|Default|Getclosed_position) (Variables|Default|Getopen_position) _door)) false false))
    (:Finished
      (Variables|Default|SetisOpen? (not (Variables|Default|GetisOpen?))))))

(event Custom|Close%20Door
  (bind _door (Timeline|open%20Door1 Reverse)
    (:Update
      (Transformation|SetRelativeLocation (Variables|Default|Getgate) (Math|Conversions|ToVector(Float) (Math|Float|Lerp (Variables|Default|Getclosed_position) (Variables|Default|Getopen_position) _door)) false false))
    (:Finished
      (Variables|Default|SetisOpen? (not (Variables|Default|GetisOpen?))))))

(event Collision|EventActorBeginOverlap
  (params (OtherActor :type Actor%20Object%20Reference))
  (|CallParentFunction OtherActor) ; This node is disabled and will not be called.\nDrag off pins to build functionality.
)

(event EventTick
  (params (DeltaSeconds :type Float%20%28single-precision%29))
  (|CallParentFunction DeltaSeconds) ; This node is disabled and will not be called.\nDrag off pins to build functionality.
)

(event EventBeginPlay
  ;[1 1 1] display text
  (bind _returnvalue (UserInterface|CreateWidget "/Game/P_Interact.P_Interact_C"))
  (Variables|Default|SetInteract%20prompt _returnvalue))

(fn ConstructionScript
  (|CallParentFunction))

(fn Interact3
  (params (Interactor :type Character%20Object%20Reference))
  (bind _open_door1 (Variables|Default|Getopen%20Door1))
  (if (not (Variables|Default|GetisOpen?))
    (Components|Timeline|SetPlayRate _open_door1 (/ 1.0 (Variables|Default|GetTime%20to%20Open%20%28s%29)))
    (CallFunction|OpenDoor)
    (else
      (Components|Timeline|SetPlayRate _open_door1 (/ 1.0 (Variables|Default|GetTime%20to%20Close%20%28s%29)))
      (CallFunction|CloseDoor)))
  (return true))